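; Co-op game mode Blueprint that responds to actor deaths by triggering a respawn.
; BeginPlay binds OnActorKilled, whose handler calls Respawn (not defined in this graph) regardless of victim or killer.
; A disconnected, never-run EQS query would find spawn locations, with its callback drawing debug spheres and spawning a BP_CoopTrackerBot at each result.
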(event Custom|OnQueryFinishedEvent_Event_0
  (params (QueryInstance :type Env%20Query%20Instance%20Blueprint%20Wrapper%20Object%20Reference) (QueryStatus :type EEnvQueryStatus%20Enum :default "Processing"))
  (switch Utilities|FlowControl|Switch|SwitchonEEnvQueryStatus QueryStatus
    (:Success
      (bind _resultlocations (AI|EQS|GetQueryResultsasLocations QueryInstance))
      (for _array_element _resultlocations
        (Rendering|Debug|DrawDebugSphere _array_element 5e+01 12 "(R=1.000000,G=0.123204,B=0.801904,A=1.000000)" 2.0 2.0)
        (Game|SpawnActorfromClass "/Game/Blueprints/BP_CoopTrackerBot.BP_CoopTrackerBot_C" (Math|Transform|MakeTransform _array_element) "AdjustIfPossibleButDontSpawnIfColliding" 0 0)))))

(event Custom|OnActorKilled_Event_0
  (params (VictimActor :type Actor%20Object%20Reference) (KillerActor :type Actor%20Object%20Reference) (KillerController :type Controller%20Object%20Reference))
  (Class|CoopGameGameModeBase|Respawn))

(event EventBeginPlay
  (EventDispatchers|AssignOnActorKilled (delegate Custom|OnActorKilled_Event_0)))

(fn ConstructionScript)