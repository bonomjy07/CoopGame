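; Co-op character Blueprint that sets up the player's HUD when play begins.
; BeginPlay creates the crosshair and health indicator widgets and adds both to the viewport.
; Two disconnected chains that would spawn a BP_CoopWeapon or BP_ProjectileWeapon and attach it to mesh sockets never run, so this graph spawns no weapon.
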(event EventBeginPlay
  ;[1 1 1] Create Crosshiar widget
  (bind _returnvalue (UserInterface|CreateWidget "/Game/UI/WBP_Crosshair.WBP_Crosshair_C"))
  (UserInterface|Viewport|AddtoViewport _returnvalue 0)
  (bind _returnvalue_2 (UserInterface|CreateWidget "/Game/UI/WBP_HealthIndicator.WBP_HealthIndicator_C"))
  (UserInterface|Viewport|AddtoViewport _returnvalue_2 0))

(fn ConstructionScript)