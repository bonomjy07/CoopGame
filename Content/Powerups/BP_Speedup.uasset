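; BP_Speedup is a powerup actor, named as a speed boost, that bobs up and down in place.
; Each Tick offsets its Z location by the scaled change in a sine of time since creation, giving a smooth hover without storing a start position.
; The OnActivated and OnExpired events are empty, so no speed effect is implemented here.
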(event EventTick
  (params (DeltaSeconds :type Float%20%28single-precision%29))
  (bind _returnvalue (Transformation|GetActorLocation))
  (bind _returnvalue_2 (Actor|GetGameTimeSinceCreation))
  (bind (_x _y _z) (Math|Vector|BreakVector _returnvalue))
  ;[1 1 1] Comment
  (Transformation|SetActorLocation (Math|Vector|MakeVector _x _y (+ _z (* (- (Math|Trig|Sin(Radians) (+ DeltaSeconds _returnvalue_2)) (Math|Trig|Sin(Radians) _returnvalue_2)) 1e+02))) false false))

(event EventOnActivated
  (params (Activator :type Actor%20Object%20Reference)))

(event EventOnExpired)

(fn ConstructionScript)