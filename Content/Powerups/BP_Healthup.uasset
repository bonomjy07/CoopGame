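; Health powerup Blueprint that heals the pawn that activates it.
; On activation it stores the activator, then heals it by a fixed amount through its CoopHealthComponent and calls ClientActivatedByPawn.
; Each powerup interval repeats that heal and call, skipping the validity check made on activation.
; The WasActivated event attaches a gold particle effect to the activator's root component.
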(event EventOnActivated
  (params (Activator :type Actor%20Object%20Reference))
  (bind _output_get (Variables|Default|SetActivator Activator))
  (|CallParentFunction _output_get)
  (Utilities|IsValid Activator
    (:Is%20Valid
      (Class|CoopHealthComponent|Heal (Actor|GetComponentbyClass _output_get "/Script/CoopGame.CoopHealthComponent") 1e+01)
      (Class|CoopPowerup|ClientActivatedbyPawn (Variables|Default|GetActivator)))))

(event EventOnPowerupInterval
  (|CallParentFunction)
  (Class|CoopHealthComponent|Heal (Actor|GetComponentbyClass (stale EventOnActivated _output_get) "/Script/CoopGame.CoopHealthComponent") 1e+01)
  (Class|CoopPowerup|ClientActivatedbyPawn (Variables|Default|GetActivator)))

(event EventOnExpired
  (|CallParentFunction))

(event EventWasActivated
  (params (Activator :type Actor%20Object%20Reference))
  (Effects|SpawnEmitterAttached "/Game/Powerups/Effects/P_gold_ore_appearance.P_gold_ore_appearance" (Variables|/Script/Engine.Actor|GetRootComponent Activator) "None" "0, 0, 0" "0, 0, 0" "1.000000,1.000000,1.000000" "SnapToTarget"))

(fn ConstructionScript)